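; AutoMortar_BP is an automatic mortar turret with a dome and barrel mesh.
; The construction script assigns the dome and barrel static meshes and sets Projectile_BP as the aiming component's projectile class.
; On BeginPlay it passes the barrel and dome to AimingComponent.Initialise as barrel and turret, leaving any aiming and firing logic to that component.
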(event EventBeginPlay
  (Class|TankAimingComponent|Initialise (Variables|Default|GetAiming%20Component) (Variables|Default|GetMortar%20Barrel) (Variables|Default|GetMortar%20Dome)))

(fn ConstructionScript
  (Components|StaticMesh|SetStaticMesh (Variables|Default|GetMortar%20Dome) "/Game/AutoMortar/mortar_dome.mortar_dome")
  (Components|StaticMesh|SetStaticMesh (Variables|Default|GetMortar%20Barrel) "/Game/AutoMortar/mortar_barrel.mortar_barrel")
  (Variables|/Script/BattleTank.TankAimingComponent|SetProjectileBP (Variables|Default|GetAiming%20Component) "/Game/Projectile/Projectile_BP.Projectile_BP_C"))